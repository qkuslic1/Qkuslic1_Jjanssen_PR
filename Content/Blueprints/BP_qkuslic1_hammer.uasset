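; Grabbable hammer actor that plays impact sounds and sparks when it strikes things.
; Pickup turns off physics and snaps it to the supplied hand component with a fixed grip offset, while Drop detaches it and restores physics.
; Collision overlaps alternate two 2D hit sounds for any actor but toggle sparks only for BP_Anvil.
; A separate OnHit event, for nail hits, sets Hit, toggles sparks and plays a success sound at world origin.
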(event OnComponentBeginOverlap(Collission)
  (params (OverlappedComponent :type Primitive%20Component%20Object%20Reference) (OtherActor :type Actor%20Object%20Reference) (OtherComp :type Primitive%20Component%20Object%20Reference) (OtherBodyIndex :type Integer) (bFromSweep :type Boolean) (SweepResult :type Hit%20Result%20Structure%20%28by%20ref%29))
  ;[1 1 1] Sparks produce when collision hits another surface
  (Utilities|FlowControl|Sequence
    (:then_0
      (Utilities|FlowControl|FlipFlop
        (:A
          (Audio|PlaySound2D "/Game/Audio/SFX_Tools/Hammer/Hammer_Hit_01_Cue.Hammer_Hit_01_Cue" 1.0 1.0 0.0 0 0))
        (:B
          (Audio|PlaySound2D "/Game/Audio/SFX_Tools/Hammer/Hammer_Hit_02_Cue.Hammer_Hit_02_Cue" 1.0 1.0 0.0 0 0))))
    (:then_1
      (Utilities|Casting|CastToBP_Anvil OtherActor)
      (Components|Activation|ToggleActive (Variables|Default|GetP_Sparks)))))

(event Custom|OnHit
  ;[1 1 1] Hammer Hits nail and sparks
  (Variables|Default|SetHit true)
  (Components|Activation|ToggleActive (Variables|Default|GetP_Sparks))
  (Audio|PlaySoundatLocation "/Game/Audio/qkuslic1_succsess_2.qkuslic1_succsess_2" "0, 0, 0" "0, 0, 0" 1.0 1.0 0.0 0 0 0))

(event EventBeginPlay
  (|CallParentFunction) ; This node is disabled and will not be called.\nDrag off pins to build functionality.
)

(event Collision|EventActorBeginOverlap
  (params (OtherActor :type Actor%20Object%20Reference))
  (|CallParentFunction OtherActor) ; This node is disabled and will not be called.\nDrag off pins to build functionality.
)

(event EventTick
  (params (DeltaSeconds :type Float%20%28single-precision%29))
  (|CallParentFunction DeltaSeconds) ; This node is disabled and will not be called.\nDrag off pins to build functionality.
)

(event EventPickup
  (params (AttachTo :type Scene%20Component%20Object%20Reference))
  ;[1 1 1] Pickup and move to hand location
  (Physics|SetSimulatePhysics (Variables|Default|GetStaticMeshComponent) false)
  (Transformation|AttachComponentToComponent (VehicleSound|GetRootComponent) AttachTo "None" "SnapToTarget" "SnapToTarget" "KeepWorld" false)
  (Transformation|SetRelativeLocationAndRotation (Variables|Default|GetStaticMeshComponent) "-3.540089,-1.072112,9.283175" "10.000011,-180.000397,0.000000" false false))

(event EventDrop
  ;[1 1 1] Pickup and move to hand location
  (Physics|SetSimulatePhysics (Variables|Default|GetStaticMeshComponent) true)
  (Transformation|DetachFromActor "KeepWorld" "KeepWorld" "KeepWorld"))

(fn ConstructionScript
  (|CallParentFunction))