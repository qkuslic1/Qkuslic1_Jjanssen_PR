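; BP_Caliper_Holder is a tool stand that snaps calipers into place when they enter its Box trigger.
; On overlap it waits, rechecking every 0.1 seconds, while the first forge metal or sword is picked up.
; It then drops the calipers, moves them to Snap, disables physics and calls attach.
; Placement and removal each fire an on/off toolstand call and update IsOnToolStand.
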(event OnComponentBeginOverlap(Box)
  (params (OverlappedComponent :type Primitive%20Component%20Object%20Reference) (OtherActor :type Actor%20Object%20Reference) (OtherComp :type Primitive%20Component%20Object%20Reference) (OtherBodyIndex :type Integer) (bFromSweep :type Boolean) (SweepResult :type Hit%20Result%20Structure%20%28by%20ref%29))
  (bind _outactors (Actor|GetAllActorsOfClass "/Game/Blueprints/BP_forge_metal.BP_forge_metal_C"))
  (bind _outactors_2 (Actor|GetAllActorsOfClass "/Game/Blueprints/BP_Sword.BP_Sword_C"))
  (if (or (Variables|/Game/Blueprints/BP_forge_metal.BP_forge_metal_C|GetObject_pickedUp? (Utilities|Array|Get(acopy) _outactors)) (Variables|/Game/Blueprints/BP_Sword.BP_Sword_C|GetObject_Pickup? (Utilities|Array|Get(acopy) _outactors_2))) :!label _label
    (Utilities|FlowControl|Delay 0.1)
    (Utilities|IsValid (Utilities|Array|Get(acopy) _outactors_2)
      (:Is%20Valid
        (Utilities|IsValid (Utilities|Array|Get(acopy) _outactors)
          (:Is%20Valid
            (goto _label)))))
    (else
      (bind _asbp_qkuslic_1_calipers (Utilities|Casting|CastToBP_qkuslic1_calipers OtherActor))
      (Default|Drop _asbp_qkuslic_1_calipers)
      (Transformation|SetActorTransform _asbp_qkuslic_1_calipers (Transformation|GetWorldTransform (Variables|Default|GetSnap)))
      (bind _output_get (Variables|Default|SetCalipers _asbp_qkuslic_1_calipers))
      (Physics|SetSimulatePhysics (Variables|/Script/Engine.StaticMeshActor|GetStaticMeshComponent _output_get) false)
      (Transformation|AttachActorToActor _asbp_qkuslic_1_calipers 0 "None" "SnapToTarget" "SnapToTarget" "KeepWorld" true)
      (Default|CallCalipersONToolStand)
      (Variables|/Game/Blueprints/BP_qkuslic1_calipers.BP_qkuslic1_calipers_C|SetARECalipersPickedUp _asbp_qkuslic_1_calipers false)
      (Variables|Default|SetIsOnToolStand? true))))

(event OnComponentEndOverlap(Box)
  (params (OverlappedComponent :type Primitive%20Component%20Object%20Reference) (OtherActor :type Actor%20Object%20Reference) (OtherComp :type Primitive%20Component%20Object%20Reference) (OtherBodyIndex :type Integer))
  ;[1 1 1] Calipers Removed
  (if (== OtherActor (Variables|Default|GetCalipers))
    (Default|CallCalipersOffToolstand)
    (Variables|Default|SetDefaultSceneRoot 0)
    (Variables|Default|SetIsOnToolStand? false)))

(fn ConstructionScript)