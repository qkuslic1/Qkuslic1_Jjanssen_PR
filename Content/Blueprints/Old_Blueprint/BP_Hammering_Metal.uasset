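; BP_Hammering_Metal is a metal piece that loses health when struck by a BP_qkuslic1_hammer actor and changes mesh once health runs out.
; Each tick it checks every hammer's collision for overlap; a DoOnce gated by delays limits hits, each costing one health and playing a sound.
; The construction script creates a dynamic material whose color briefly flashes red on hit.
; At zero health, a short delay precedes the swap to an anvil stand mesh.
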(event EventBeginPlay
  ;[1 1 1] Health System and Static Mesh Swap
)

(event EventTick
  (params (DeltaSeconds :type Float%20%28single-precision%29))
  (bind _damagecolor (Variables|Default|GetDamageColor))
  ;[1 1 1] Health System and Static Mesh Swap
  (bind _outactors (Actor|GetAllActorsOfClass "/Game/Blueprints/BP_qkuslic1_hammer.BP_qkuslic1_hammer_C"))
  (for _array_element _outactors
    (if (Collision|IsOverlappingActor (Variables|/Game/Blueprints/BP_qkuslic1_hammer.BP_qkuslic1_hammer_C|GetCollission _array_element) self :!class /Script/Engine.PrimitiveComponent)
      (if (>= (Variables|Default|GetHealth) 1)
        (Development|PrintString "Hit")
        (Utilities|FlowControl|DoOnce false :!label _label
          (:Completed
            (Utilities|FlowControl|Delay 0.0)
            (Variables|Default|SetHealth (- (Variables|Default|GetHealth) 1))
            (Audio|PlaySound2D "/Game/Audio/qkuslic1_Gliss.qkuslic1_Gliss" 1.0 1.0 0.0 0 0)
            (Rendering|Material|SetVectorParameterValue _damagecolor "Color" "(R=1.000000,G=0.000000,B=0.012273,A=1.000000)" :!class /Script/Engine.MaterialInstanceDynamic)
            (Utilities|FlowControl|Delay 0.2)
            (Rendering|Material|SetVectorParameterValue :self _damagecolor :ParameterName "Color" :!class /Script/Engine.MaterialInstanceDynamic)
            (Utilities|FlowControl|Delay 0.1)
            (goto _label Reset)))
        (else
          (Utilities|FlowControl|Delay 0.3)
          (Components|StaticMesh|SetStaticMesh (Variables|Default|GetHammered_Metal) "/Game/Geometry/Meshes/Tools/SM_jjanssen_Anvil_Stand_High.SM_jjanssen_Anvil_Stand_High"))))))

(fn ConstructionScript
  ;[1 1 1] Creates Dynamic Material
  (bind _returnvalue (Rendering|Material|CreateDynamicMaterialInstance (Variables|Default|GetHammered_Metal) 0 "/Game/castiron.castiron" "" :!class /Script/Engine.PrimitiveComponent))
  (Variables|Default|SetDamageColor _returnvalue))