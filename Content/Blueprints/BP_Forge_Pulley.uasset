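; VR forge pulley that a motion controller grabs and slides along local Z, built on drawer logic.
; Overlap sets hover, Pickup stores a grab offset, and Tick moves DrawerRoot with the controller, clamped to DrawerLength.
; Drop fires BP_Forge with a sound if ore is inside.
; A gated friction-coasting simulation exists, but release calls StopDrawerPhysics, and nothing here calls StartSimulateDrawer.
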(event OnComponentBeginOverlap(HandleCollision)
  (params (OverlappedComponent :type Primitive%20Component%20Object%20Reference) (OtherActor :type Actor%20Object%20Reference) (OtherComp :type Primitive%20Component%20Object%20Reference) (OtherBodyIndex :type Integer) (bFromSweep :type Boolean) (SweepResult :type Hit%20Result%20Structure%20%28by%20ref%29))
  ;[1 1 1] On/Off Hover
  (Utilities|Casting|CastToBP_MotionController OtherActor)
  (CallFunction|OnHover02))

(event OnComponentEndOverlap(HandleCollision)
  (params (OverlappedComponent :type Primitive%20Component%20Object%20Reference) (OtherActor :type Actor%20Object%20Reference) (OtherComp :type Primitive%20Component%20Object%20Reference) (OtherBodyIndex :type Integer))
  ;[1 1 1] On/Off Hover
  (Utilities|Casting|CastToBP_MotionController OtherActor)
  (CallFunction|OffHover))

(event Custom|StartSimulateDrawer
  (params (InitialVelocity :type Float%20%28single-precision%29))
  (bind _drawerroot (Variables|Default|GetDrawerRoot))
  (bind _relativelocation (Variables|/Script/Engine.SceneComponent|GetRelativeLocation _drawerroot))
  ;[1 1 1] Simulate Drawer
  (Variables|Default|SetDrawerInitialVelocity InitialVelocity)
  (Variables|Default|SetDrawerTimeSinceLetGo 0.0)
  (Utilities|FlowControl|Gate true) ; enters at Open
)

(event Custom|StopDrawerPhysics
  (params (InitialVelocity :type Float%20%28single-precision%29))
  (bind _drawerroot (Variables|Default|GetDrawerRoot))
  (bind _relativelocation (Variables|/Script/Engine.SceneComponent|GetRelativeLocation _drawerroot))
  ;[1 1 1] Simulate Drawer
  (Utilities|FlowControl|Gate true) ; enters at Close
)

(event Custom|Reset%20Location
  (Variables|Default|SetIsResettingLocation? true)
  (Variables|Default|SetInitialLocation "0, 0, 0"))

(event EventBeginPlay
  ;[1 1 1] Initialize
  (Variables|Default|SetInitialLocation (Variables|/Script/Engine.SceneComponent|GetRelativeLocation (Variables|Default|GetDrawerRoot))))

(event EventPickup
  (params (AttachTo :type Scene%20Component%20Object%20Reference))
  ;[1 1 1] Grab/Drop
  (if (Variables|Default|GetHovered?)
    (Variables|Default|SetGrabbed true)
    (bind _output_get (Variables|Default|SetPointTo AttachTo))
    (Variables|Default|SetGrabOffset (- (.Z (Math|Vector|BreakVector (Math|Transform|InverseTransformLocation (Transformation|GetActorTransform) (Transformation|GetWorldLocation _output_get)))) (.z (Variables|/Script/Engine.SceneComponent|GetRelativeLocation (Variables|Default|GetDrawerRoot)))))))

(event EventDrop
  (Variables|Default|SetGrabbed false)
  ;[1 1 1] Grab/Drop
  (CallFunction|DragDrawerStop)
  (bind _outactors (Actor|GetAllActorsOfClass "/Game/Blueprints/BP_Forge.BP_Forge_C"))
  (if (Variables|/Game/Blueprints/BP_Forge.BP_Forge_C|GetOre%20is%20in%20forge (Utilities|Array|Get(acopy) _outactors))
    (Variables|Default|SetLeverPulled? true)
    (Audio|PlaySound2D "/Game/Audio/SFX_Tools/Forge/frw_Cue.frw_Cue" 1.0 1.0 0.0 0 0) ; change sound to pull noise later
    (bind _outactors_2 (Actor|GetAllActorsOfClass "/Game/Blueprints/BP_Forge.BP_Forge_C"))
    (Default|CallForgeisFired (Utilities|Array|Get(acopy) _outactors_2))
    (Variables|Default|SetForgeIsFired true)))

(event EventTick
  (params (DeltaSeconds :type Float%20%28single-precision%29))
  (bind _drawerroot (Variables|Default|GetDrawerRoot))
  (bind _relativelocation (Variables|/Script/Engine.SceneComponent|GetRelativeLocation _drawerroot))
  ;[1 1 1] SituationalFunctions
  (Utilities|FlowControl|Sequence
    (:then_0
      (if (Variables|Default|GetGrabbed)
        (CallFunction|DragDrawer)))
    (:then_2
      ;[1 1 1] Simulate Drawer
      (Utilities|FlowControl|Gate true
        (:Exit
          (Variables|Default|SetDrawerTimeSinceLetGo (+ (Variables|Default|GetDrawerTimeSinceLetGo) DeltaSeconds))
          (Transformation|SetRelativeLocation (Variables|Default|GetDrawerRoot) (Math|Vector|MakeVector 0.0 0.0 (Math|Float|Clamp(Float) (+ (Variables|Default|GetCurrentDrawerPosition) (- (* (Variables|Default|GetDrawerInitialVelocity) (Variables|Default|GetDrawerTimeSinceLetGo)) (* 0.5 (* (Variables|Default|GetDrawerFriction) 9.8e+02) (Math|Float|Square (Variables|Default|GetDrawerTimeSinceLetGo)) (Math|Float|Sign(Float) (Variables|Default|GetDrawerInitialVelocity))))) 0.0 (Variables|Default|GetDrawerLength))) false false)
          (if (Math|Boolean|ORBoolean (select (<= (Variables|Default|GetDrawerInitialVelocity) 0.0) (> (- (Variables|Default|GetDrawerInitialVelocity) (* (* (Variables|Default|GetDrawerFriction) 9.8e+02) (Variables|Default|GetDrawerTimeSinceLetGo) (Math|Float|Sign(Float) (Variables|Default|GetDrawerInitialVelocity)))) 0.0) (<= (- (Variables|Default|GetDrawerInitialVelocity) (* (* (Variables|Default|GetDrawerFriction) 9.8e+02) (Variables|Default|GetDrawerTimeSinceLetGo) (Math|Float|Sign(Float) (Variables|Default|GetDrawerInitialVelocity)))) 0.0)) (Math|Float|NearlyEqual(Float) (.z _relativelocation) 0.0 0.01) (Math|Float|NearlyEqual(Float) (.z _relativelocation) (Variables|Default|GetDrawerLength) 0.01))
            (CallFunction|StopDrawerPhysics 0.0)))))))

(fn ConstructionScript)

(fn OnHover02
  (Variables|Default|SetHovered? true))

(fn OffHover
  (Variables|Default|SetHovered? false))

(fn DragDrawer
  (bind _returnvalue (Transformation|GetActorTransform))
  (bind _pointto (Variables|Default|GetPointTo))
  (bind _graboffset (Variables|Default|GetGrabOffset))
  (bind _drawerlength (Variables|Default|GetDrawerLength))
  (bind _returnvalue_2 (Transformation|GetWorldLocation _pointto))
  (bind _returnvalue_3 (Math|Transform|InverseTransformLocation _returnvalue _returnvalue_2))
  (bind _z (Math|Vector|BreakVector _returnvalue_3))
  (bind _returnvalue_4 (- _z _graboffset))
  (bind _returnvalue_5 (Math|Float|Clamp(Float) _returnvalue_4 0.0 _drawerlength))
  ;[1 1 1] SetRotation
  (Variables|Default|SetPreviousDrawerPosition (Variables|Default|GetCurrentDrawerPosition))
  (Variables|Default|SetCurrentDrawerPosition _returnvalue_5)
  (Variables|Default|SetCurrentDrawerPositionNormalized (/ _returnvalue_5 (Variables|Default|GetDrawerLength)))
  (Transformation|SetRelativeLocation (Variables|Default|GetDrawerRoot) (Math|Vector|MakeVector 0.0 0.0 (Variables|Default|GetCurrentDrawerPosition)) false false))

(fn DragDrawerStop
  (CallFunction|StopDrawerPhysics (/ (- (Variables|Default|GetCurrentDrawerPosition) (Variables|Default|GetPreviousDrawerPosition)) (Utilities|Time|GetWorldDeltaSeconds))))

(fn CanPickup
  (return false))

(fn OnDrag
  (params (Interactor :type World%20Interactor%20Object%20Reference))
  (return false))

(fn OnDragEnd
  (params (Interactor :type World%20Interactor%20Object%20Reference))
  (return false))

(fn OnDragStart
  (params (Interactor :type World%20Interactor%20Object%20Reference))
  (return false))

(fn OnDrop
  (params (Interactor :type World%20Interactor%20Object%20Reference))
  (return false))

(fn OnHover
  (params (Interactor :type World%20Interactor%20Object%20Reference))
  (return false))

(fn OnPickup
  (params (Interactor :type World%20Interactor%20Object%20Reference))
  (return false))

(fn OnUnHover
  (params (Interactor :type World%20Interactor%20Object%20Reference))
  (return false))

(fn OnUse
  (params (Interactor :type World%20Interactor%20Object%20Reference))
  (return false))