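; Water trough that quenches a sword, apparently a cooling step in a smithing sequence.
; When a BP_Sword with ObjectPickup set overlaps Collision, it plays a steam sound, activates steam particles and hides the sword.
; After a short delay it spawns a BP_Sword_Dull at the SwordGetter component's transform and sets CooledOff.
; DoOnce gates make the quench a one-time event.
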(event OnComponentBeginOverlap(Collision)
  (params (OverlappedComponent :type Primitive%20Component%20Object%20Reference) (OtherActor :type Actor%20Object%20Reference) (OtherComp :type Primitive%20Component%20Object%20Reference) (OtherBodyIndex :type Integer) (bFromSweep :type Boolean) (SweepResult :type Hit%20Result%20Structure%20%28by%20ref%29))
  (bind _sword_getter (Variables|Default|GetSword_Getter))
  ;[1 1 1] Spawns Steam Once Metal (After Swap Static Mesh) is activated
  (bind _asbp_sword (Utilities|Casting|CastToBP_Sword OtherActor))
  (if (Variables|/Game/Blueprints/BP_Sword.BP_Sword_C|GetObject_Pickup? _asbp_sword)
    (Utilities|FlowControl|DoOnce false
      (:Completed
        (Audio|PlaySound2D "/Game/Audio/SFX_Tools/Water_Trough/Steam_02_Cue.Steam_02_Cue" 1.0 1.0 0.0 0 0)
        (Components|Activation|Activate (Variables|Default|GetP_Steam) false)
        (Utilities|FlowControl|DoOnce false
          (:Completed
            (Rendering|SetActorHiddenInGame _asbp_sword true)
            ;[1 1 1] Spawns Sword in water
            (Utilities|FlowControl|Delay 0.2)
            (Game|SpawnActorfromClass "/Game/Blueprints/BP_Sword_Dull.BP_Sword_Dull_C" (Math|Transform|MakeTransform (Transformation|GetWorldLocation _sword_getter) (Transformation|GetWorldRotation _sword_getter)) "Undefined" 0 0)
            (Variables|Default|SetCooledOff? true)))))))

(event EventBeginPlay)

(event Collision|EventActorBeginOverlap
  (params (OtherActor :type Actor%20Object%20Reference)))

(event EventTick
  (params (DeltaSeconds :type Float%20%28single-precision%29)))

(fn ConstructionScript)