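; VR forge actor that turns an iron ingot dropped into its trigger box into forge metal.
; An ingot overlap plays a success sound, increments the motion controller pawn's counter and flags that ore is in the forge.
; It then polls the first BP_Forge_Pulley on a short Delay loop until that reports the forge is fired.
; A DoOnce then toggles lava and its light, activates fire, hides the ingot and spawns the metal at RoddGetter.
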(event OnComponentBeginOverlap(Box)
  (params (OverlappedComponent :type Primitive%20Component%20Object%20Reference) (OtherActor :type Actor%20Object%20Reference) (OtherComp :type Primitive%20Component%20Object%20Reference) (OtherBodyIndex :type Integer) (bFromSweep :type Boolean) (SweepResult :type Hit%20Result%20Structure%20%28by%20ref%29))
  (bind _rodd_getter (Variables|Default|GetRodd%20Getter))
  (bind _asbp_jjanssen_iron_ingot (Utilities|Casting|CastToBP_jjanssen_Iron_Ingot OtherActor))
  (Audio|PlaySound2D "/Game/Audio/qkuslic1_succsess_2_Cue.qkuslic1_succsess_2_Cue" 1.0 1.0 0.0 0 0)
  (bind _asmotion_controller_pawn (Utilities|Casting|CastToMotionControllerPawn (Game|Player|GetPlayerPawn 0)))
  (bind _output_get (Variables|/Game/VirtualRealityBP/Blueprints/MotionControllerPawn.MotionControllerPawn_C|SetCounter _asmotion_controller_pawn (+ (Variables|/Game/VirtualRealityBP/Blueprints/MotionControllerPawn.MotionControllerPawn_C|GetCounter _asmotion_controller_pawn) 1)))
  (if (not (<= _output_get 0))
    (Default|CallOreIsinForge)
    (Variables|Default|SetOre%20is%20in%20forge true)
    (bind _outactors (Actor|GetAllActorsOfClass "/Game/Blueprints/BP_Forge_Pulley.BP_Forge_Pulley_C"))
    (if (Variables|/Game/Blueprints/BP_Forge_Pulley.BP_Forge_Pulley_C|GetForgeIsFired (Utilities|Array|Get(acopy) _outactors)) :!label _label
      (Utilities|FlowControl|DoOnce false
        (:Completed
          (Rendering|ToggleVisibility (Variables|Default|GetLava) false)
          (Rendering|ToggleVisibility (Variables|Default|GetLava_Light) false)
          (Components|Activation|SetActive (Variables|Default|GetFire) true false)
          (Rendering|SetActorHiddenInGame _asbp_jjanssen_iron_ingot true)
          (Game|SpawnActorfromClass "/Game/Blueprints/BP_forge_metal.BP_forge_metal_C" (Math|Transform|MakeTransform (Transformation|GetWorldLocation _rodd_getter) (Transformation|GetWorldRotation _rodd_getter)) "Undefined" 0 0)))
      (else
        (Utilities|FlowControl|Delay 0.2 :!label _label_2)
        (Utilities|IsValid (Utilities|Array|Get(acopy) _outactors)
          (:Is%20Valid
            (goto _label))
          (:Is%20Not%20Valid
            (goto _label_2)))))))

(event Collision|EventActorBeginOverlap
  (params (OtherActor :type Actor%20Object%20Reference)))

(event EventTick
  (params (DeltaSeconds :type Float%20%28single-precision%29)))

(fn ConstructionScript)