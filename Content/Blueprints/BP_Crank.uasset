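; BP_Crank is an interactable crank lever that a player drags to fire its Turned event.
; One interactor at a time drags it, and its position in actor space is converted through Atan2 into a clamped lever pitch.
; Reaching the activation pitch fires the event and starts a timeline that lerps the lever back to its BeginPlay rotation, ignoring drag until finished.
; Releasing the drag also resets the lever, and pickup is disabled.
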(event Custom|ResetRotation
  (Variables|Default|SetIsResettingRotation true)
  (Variables|Default|SetInitialResetRotation (Variables|/Script/Engine.SceneComponent|GetRelativeRotation (Variables|Default|GetLeverRotate)))
  (bind _alpha (Timeline|ResetRotationTimeline Play)
    (:Update
      (Transformation|SetRelativeRotation (Variables|Default|GetLeverRotate) (Math|Rotator|Lerp(Rotator) (Variables|Default|GetInitialResetRotation) (Variables|Default|GetInitialLeverRotation) _alpha) false false))
    (:Finished
      (Variables|Default|SetIsResettingRotation false))))

(event EventBeginPlay
  (Variables|Default|SetInitialLeverRotation (Variables|/Script/Engine.SceneComponent|GetRelativeRotation (Variables|Default|GetLeverRotate))))

(fn ConstructionScript)

(fn CanPickup
  (return false))

(fn OnDrag
  (params (Interactor :type World%20Interactor%20Object%20Reference))
  (bind _returnvalue (Transformation|GetActorTransform))
  (bind _currentinteractor (Variables|Default|GetCurrentInteractor))
  (bind _returnvalue_2 (Transformation|GetWorldLocation _currentinteractor))
  (bind _returnvalue_3 (Math|Transform|InverseTransformLocation _returnvalue _returnvalue_2))
  (bind _returnvalue_4 (Math|Vector|UnrotateVector _returnvalue_3 "90.000000,0.000000,0.000000"))
  (if (== Interactor (Variables|Default|GetCurrentInteractor))
    (if (not (Variables|Default|GetIsResettingRotation))
      (bind _output_get (Variables|Default|SetCurrentPitch (Math|Float|Clamp(Float) (Class|KismetMathLibrary|DegAtan2 (.z _returnvalue_4) (.x _returnvalue_4)) (Variables|Default|GetMinPitch) (Variables|Default|GetMaxPitch))))
      (Transformation|SetRelativeRotation (Variables|Default|GetLeverRotate) (Math|Rotator|MakeRotator 0.0 _output_get 0.0) false false)
      (if (== (Variables|Default|GetCurrentPitch) (Variables|Default|GetActivationPitch))
        (CallFunction|ResetRotation)
        (Default|CallTurned)
        (return false)
        (else
          (return false)))
      (else
        (return false)))
    (else
      (return false))))

(fn OnDragEnd
  (params (Interactor :type World%20Interactor%20Object%20Reference))
  (if (== Interactor (Variables|Default|GetCurrentInteractor))
    (CallFunction|ResetRotation)
    (Variables|Default|SetCurrentInteractor 0))
  (return false))

(fn OnDragStart
  (params (Interactor :type World%20Interactor%20Object%20Reference))
  (Utilities|IsValid (Variables|Default|GetCurrentInteractor)
    (:Is%20Valid
      _)
    (:Is%20Not%20Valid
      (Variables|Default|SetCurrentInteractor Interactor)))
  (return false))

(fn OnDrop
  (params (Interactor :type World%20Interactor%20Object%20Reference))
  (return false))

(fn OnHover
  (params (Interactor :type World%20Interactor%20Object%20Reference))
  (return false))

(fn OnPickup
  (params (Interactor :type World%20Interactor%20Object%20Reference))
  (return false))

(fn OnUnHover
  (params (Interactor :type World%20Interactor%20Object%20Reference))
  (return false))

(fn OnUse
  (params (Interactor :type World%20Interactor%20Object%20Reference))
  (return false))