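; BP_jjanssen_Iron_Ingot is an iron ingot actor that motion controllers can pick up and drop.
; Pickup disables mesh physics and attaches the root to the supplied component; Drop restores physics and detaches it.
; Both events set IsOrePickedup on the first BP_MotionController found in the world, not necessarily the one holding it.
; The other interaction functions are stubs returning false, and the ingot counter logic is unconnected.
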(event Collision|EventActorBeginOverlap
  (params (OtherActor :type Actor%20Object%20Reference)))

(event EventTick
  (params (DeltaSeconds :type Float%20%28single-precision%29)))

(event EventPickup
  (params (AttachTo :type Scene%20Component%20Object%20Reference))
  (bind _outactors (Actor|GetAllActorsOfClass "/Game/VirtualRealityBP/Blueprints/BP_MotionController.BP_MotionController_C"))
  (Variables|/Game/VirtualRealityBP/Blueprints/BP_MotionController.BP_MotionController_C|SetIsOrePickedup? (Utilities|Array|Get(acopy) _outactors) true)
  (Physics|SetSimulatePhysics (Variables|Debug|GetStaticMeshComponent) false)
  (Transformation|AttachComponentToComponent (VehicleSound|GetRootComponent) AttachTo "None" "KeepWorld" "KeepWorld" "KeepWorld" false))

(event EventDrop
  (bind _outactors (Actor|GetAllActorsOfClass "/Game/VirtualRealityBP/Blueprints/BP_MotionController.BP_MotionController_C"))
  (Variables|/Game/VirtualRealityBP/Blueprints/BP_MotionController.BP_MotionController_C|SetIsOrePickedup? (Utilities|Array|Get(acopy) _outactors) false)
  (Physics|SetSimulatePhysics (Variables|Debug|GetStaticMeshComponent) true)
  (Transformation|DetachFromActor "KeepWorld" "KeepWorld" "KeepWorld"))

(fn ConstructionScript)

(fn CanPickup
  (return false))

(fn OnDrag
  (params (Interactor :type World%20Interactor%20Object%20Reference))
  (return false))

(fn OnDragEnd
  (params (Interactor :type World%20Interactor%20Object%20Reference))
  (return false))

(fn OnDragStart
  (params (Interactor :type World%20Interactor%20Object%20Reference))
  (return false))

(fn OnDrop
  (params (Interactor :type World%20Interactor%20Object%20Reference))
  (return false))

(fn OnHover
  (params (Interactor :type World%20Interactor%20Object%20Reference))
  (return false))

(fn OnPickup
  (params (Interactor :type World%20Interactor%20Object%20Reference))
  (return false))

(fn OnUnHover
  (params (Interactor :type World%20Interactor%20Object%20Reference))
  (return false))

(fn OnUse
  (params (Interactor :type World%20Interactor%20Object%20Reference))
  (return false))