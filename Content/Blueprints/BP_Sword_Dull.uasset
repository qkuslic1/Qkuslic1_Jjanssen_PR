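; Dull sword prop that can be picked up and sharpened on a crank-driven grindstone.
; Pickup attaches it to the given component without physics, and Drop detaches it with physics restored.
; Tick polls every BP_Crank_2, draining Health at a throttled rate while its rotating grindstone registers a hit, then swaps once to the pristine mesh with success sound and particles.
; The caliper attach loop is unwired, and interaction functions are stubs returning false.
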(event OnComponentBeginOverlap(StaticMeshComponent)
  (params (OverlappedComponent :type Primitive%20Component%20Object%20Reference) (OtherActor :type Actor%20Object%20Reference) (OtherComp :type Primitive%20Component%20Object%20Reference) (OtherBodyIndex :type Integer) (bFromSweep :type Boolean) (SweepResult :type Hit%20Result%20Structure%20%28by%20ref%29))
  ;[1 1 1] Caliper Pickup Interaction
)

(event EventBeginPlay)

(event Collision|EventActorBeginOverlap
  (params (OtherActor :type Actor%20Object%20Reference)))

(event EventPickup
  (params (AttachTo :type Scene%20Component%20Object%20Reference))
  ;[1 1 1] Pickup/Drop
  (Physics|SetSimulatePhysics (Variables|Debug|GetStaticMeshComponent) false)
  (Transformation|AttachComponentToComponent (VehicleSound|GetRootComponent) AttachTo "None" "SnapToTarget" "SnapToTarget" "KeepWorld" false)
  (Variables|Default|SetSwordGrabbed? true)
  (Transformation|SetRelativeLocationAndRotation (Variables|Debug|GetStaticMeshComponent) "-0.531057,-1.000000,38.451900" "-85.000000,180.000000,180.000000" false false))

(event EventDrop
  ;[1 1 1] Pickup/Drop
  (Physics|SetSimulatePhysics (Variables|Debug|GetStaticMeshComponent) true)
  (Transformation|DetachFromActor "KeepWorld" "KeepWorld" "KeepWorld")
  (Variables|Default|SetSwordGrabbed? false))

(event EventTick
  (params (DeltaSeconds :type Float%20%28single-precision%29))
  ;[1 1 1] Health System for Sword While Grinding
  (bind _outactors (Actor|GetAllActorsOfClass "/Game/Blueprints/BP_Crank_2.BP_Crank_2_C"))
  (for _array_element _outactors
    (if (Collision|IsOverlappingActor (Variables|/Game/Blueprints/BP_Crank_2.BP_Crank_2_C|GetGrindStone_Collision _array_element) self :!class /Script/Engine.PrimitiveComponent)
      (if (Variables|/Game/Blueprints/BP_Crank_2.BP_Crank_2_C|GetIsRotating? _array_element)
        (if (Variables|/Game/Blueprints/BP_Crank_2.BP_Crank_2_C|GetHit _array_element)
          (if (>= (Variables|Default|GetHealth) 1)
            (Utilities|FlowControl|DoOnce false :!label _label
              (:Completed
                (Utilities|FlowControl|Delay 0.0)
                (Variables|Default|SetHealth (- (Variables|Default|GetHealth) 1))
                (Utilities|FlowControl|Delay 0.2)
                (goto _label Reset)))
            (else
              (Utilities|FlowControl|DoOnce false
                (:Completed
                  (Utilities|FlowControl|Delay 0.3)
                  (Components|StaticMesh|SetStaticMesh (Variables|Debug|GetStaticMeshComponent) "/Game/Geometry/Meshes/Tools/jjanssen_Sword_Pristine_High.jjanssen_Sword_Pristine_High")
                  (Variables|Default|SetSwitch? true)
                  (Audio|PlaySound2D "/Game/Audio/qkuslic1_succsess_2_Cue.qkuslic1_succsess_2_Cue" 1.0 1.0 0.0 0 0)
                  (Components|Activation|Activate (Variables|Default|GetParticle2) false))))))))))

(fn ConstructionScript)

(fn CanPickup
  (return false))

(fn OnDrag
  (params (Interactor :type World%20Interactor%20Object%20Reference))
  (return false))

(fn OnDragEnd
  (params (Interactor :type World%20Interactor%20Object%20Reference))
  (return false))

(fn OnDragStart
  (params (Interactor :type World%20Interactor%20Object%20Reference))
  (return false))

(fn OnDrop
  (params (Interactor :type World%20Interactor%20Object%20Reference))
  (return false))

(fn OnHover
  (params (Interactor :type World%20Interactor%20Object%20Reference))
  (return false))

(fn OnPickup
  (params (Interactor :type World%20Interactor%20Object%20Reference))
  (return false))

(fn OnUnHover
  (params (Interactor :type World%20Interactor%20Object%20Reference))
  (return false))

(fn OnUse
  (params (Interactor :type World%20Interactor%20Object%20Reference))
  (return false))