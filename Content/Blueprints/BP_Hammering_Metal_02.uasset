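; BP_Hammering_Metal_02 is a VR metal rod that can be held with calipers, with unfinished or disconnected logic for hammering it into a sword.
; Overlapping the calipers starts a per-frame Delay loop that attaches or releases the mesh according to the motion controller pawn's CalipersUsed flag.
; Construction creates a dynamic material for damage flashes, but the hammer-hit health countdown, flash and BP_Sword spawn never run.
; Pickup events and interaction functions are empty stubs.
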(event OnComponentBeginOverlap(StaticMeshComponent)
  (params (OverlappedComponent :type Primitive%20Component%20Object%20Reference) (OtherActor :type Actor%20Object%20Reference) (OtherComp :type Primitive%20Component%20Object%20Reference) (OtherBodyIndex :type Integer) (bFromSweep :type Boolean) (SweepResult :type Hit%20Result%20Structure%20%28by%20ref%29))
  ;[1 1 1] Caliper Pickup Interaction
  (bind _asbp_qkuslic_1_calipers (Utilities|Casting|CastToBP_qkuslic1_calipers OtherActor))
  (bind _outactors (Actor|GetAllActorsOfClass "/Game/VirtualRealityBP/Blueprints/MotionControllerPawn.MotionControllerPawn_C"))
  (if (Variables|/Game/VirtualRealityBP/Blueprints/MotionControllerPawn.MotionControllerPawn_C|GetCalipersUsed (Utilities|Array|Get(acopy) _outactors)) :!label _label
    (Physics|SetSimulatePhysics (Variables|Debug|GetStaticMeshComponent) false)
    (Transformation|AttachComponentToComponent (Variables|Debug|GetStaticMeshComponent) (Variables|/Game/Blueprints/BP_qkuslic1_calipers.BP_qkuslic1_calipers_C|GetSphere _asbp_qkuslic_1_calipers) "None" "SnapToTarget" "SnapToTarget" "KeepWorld" true)
    (Variables|Default|SetObject_pickedUp? true)
    (Utilities|FlowControl|Delay 0.0 :!label _label_2)
    (Utilities|IsValid (Utilities|Array|Get(acopy) _outactors)
      (:Is%20Valid
        (goto _label))
      (:Is%20Not%20Valid
        (goto _label_2)))
    (else
      (Physics|SetSimulatePhysics (Variables|Debug|GetStaticMeshComponent) true)
      (Transformation|DetachFromComponent (Variables|Debug|GetStaticMeshComponent) "KeepWorld" "KeepWorld" "KeepWorld" true)
      (Variables|Default|SetObject_pickedUp? false)
      (Utilities|FlowControl|Delay 0.0 :!label _label_3)
      (Utilities|IsValid (Utilities|Array|Get(acopy) _outactors)
        (:Is%20Valid
          (goto _label))
        (:Is%20Not%20Valid
          (goto _label_3))))))

(event EventBeginPlay
  ;[1 1 1] Health System and Static Mesh Swap
)

(event EventPickup
  (params (AttachTo :type Scene%20Component%20Object%20Reference))
  ;[1 1 1] Pickup/Drop
)

(event EventDrop
  ;[1 1 1] Pickup/Drop
)

(event EventTick
  (params (DeltaSeconds :type Float%20%28single-precision%29))
  ;[1 1 1] Health System and Static Mesh Swap
)

(fn ConstructionScript
  (bind _returnvalue (Rendering|Material|CreateDynamicMaterialInstance (Variables|Debug|GetStaticMeshComponent) 0 "/Game/Materials/M_MetalRod/M_MetalRodPipe.M_MetalRodPipe" "None" :!class /Script/Engine.PrimitiveComponent))
  (Variables|Default|SetDamageColor _returnvalue))

(fn CanPickup
  (return false))

(fn OnDrag
  (params (Interactor :type World%20Interactor%20Object%20Reference))
  (return false))

(fn OnDragEnd
  (params (Interactor :type World%20Interactor%20Object%20Reference))
  (return false))

(fn OnDragStart
  (params (Interactor :type World%20Interactor%20Object%20Reference))
  (return false))

(fn OnDrop
  (params (Interactor :type World%20Interactor%20Object%20Reference))
  (return false))

(fn OnHover
  (params (Interactor :type World%20Interactor%20Object%20Reference))
  (return false))

(fn OnPickup
  (params (Interactor :type World%20Interactor%20Object%20Reference))
  (return false))

(fn OnUnHover
  (params (Interactor :type World%20Interactor%20Object%20Reference))
  (return false))

(fn OnUse
  (params (Interactor :type World%20Interactor%20Object%20Reference))
  (return false))