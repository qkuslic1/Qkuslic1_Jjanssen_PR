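; BP_Anvil is a forging anvil that turns a placed piece of metal into a sword through hammering.
; A BP_forge_metal entering the Box is hidden once, toggles the IronRod mesh's visibility, and fires RodIsPlaced.
; Tick then polls all hammer actors for overlap, decrementing Health behind a delay-reset DoOnce.
; Once Health is depleted, the next overlap toggles the rod again, spawns BP_Sword, and sets Switch.
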(event OnComponentBeginOverlap(Box)
  (params (OverlappedComponent :type Primitive%20Component%20Object%20Reference) (OtherActor :type Actor%20Object%20Reference) (OtherComp :type Primitive%20Component%20Object%20Reference) (OtherBodyIndex :type Integer) (bFromSweep :type Boolean) (SweepResult :type Hit%20Result%20Structure%20%28by%20ref%29))
  (bind _asbp_forge_metal (Utilities|Casting|CastToBP_forge_metal OtherActor :!label _label))
  (Utilities|IsValid _asbp_forge_metal
    (:Is%20Valid
      (Utilities|FlowControl|DoOnce false
        (:Completed
          (Rendering|SetActorHiddenInGame _asbp_forge_metal true)
          (Rendering|ToggleVisibility (Variables|Default|GetIronRod) false)
          (Default|CallRodIsPlaced)
          (Variables|Default|SetIsRodON true))))
    (:Is%20Not%20Valid
      (goto _label))))

(event EventTick
  (params (DeltaSeconds :type Float%20%28single-precision%29))
  (bind _staticmesh (Variables|Default|GetStaticMesh))
  (if (Variables|Default|GetIsRodON)
    (bind _outactors (Actor|GetAllActorsOfClass "/Game/Blueprints/BP_qkuslic1_hammer.BP_qkuslic1_hammer_C"))
    (for _array_element _outactors
      (if (Collision|IsOverlappingActor (Variables|/Game/Blueprints/BP_qkuslic1_hammer.BP_qkuslic1_hammer_C|GetCollission _array_element) self :!class /Script/Engine.PrimitiveComponent)
        (if (>= (Variables|Default|GetHealth) 1)
          (Utilities|FlowControl|DoOnce false :!label _label
            (:Completed
              (Utilities|FlowControl|Delay 0.0)
              (Variables|Default|SetHealth (- (Variables|Default|GetHealth) 1))
              (Utilities|FlowControl|Delay 0.2)
              (Utilities|FlowControl|Delay 0.1)
              (goto _label Reset)))
          (else
            (Utilities|FlowControl|DoOnce false
              (:Completed
                ;[1 1 1] Toggle Visibility to Hammered Metal and Spawns Sword, checks to if hammer changed to sword
                (Utilities|FlowControl|Delay 0.3)
                (Rendering|ToggleVisibility (Variables|Default|GetIronRod) false)
                (Game|SpawnActorfromClass "/Game/Blueprints/BP_Sword.BP_Sword_C" (Math|Transform|MakeTransform (Transformation|GetWorldLocation _staticmesh) (Transformation|GetWorldRotation _staticmesh)) "Undefined" 0 0)
                (Variables|Default|SetSwitch true)))))))))

(fn ConstructionScript)