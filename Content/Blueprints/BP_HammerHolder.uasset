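; BP_HammerHolder is a holder that snaps a BP_qkuslic1_hammer into place when it enters the Box trigger.
; On overlap it forces the hammer to drop, moves it to the StaticMesh transform, disables its physics, attaches it and fires HammerIn.
; When the stored hammer leaves the box, it fires HammerNotIn and sets DefaultSceneRoot to None, leaving the Hammer reference set.
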(event OnComponentBeginOverlap(Box)
  (params (OverlappedComponent :type Primitive%20Component%20Object%20Reference) (OtherActor :type Actor%20Object%20Reference) (OtherComp :type Primitive%20Component%20Object%20Reference) (OtherBodyIndex :type Integer) (bFromSweep :type Boolean) (SweepResult :type Hit%20Result%20Structure%20%28by%20ref%29))
  (bind _asbp_qkuslic_1_hammer (Utilities|Casting|CastToBP_qkuslic1_hammer OtherActor))
  (Default|Drop _asbp_qkuslic_1_hammer)
  (Transformation|SetActorTransform _asbp_qkuslic_1_hammer (Transformation|GetWorldTransform (Variables|Default|GetStaticMesh)))
  (bind _output_get (Variables|Default|SetHammer _asbp_qkuslic_1_hammer))
  (Physics|SetSimulatePhysics (Variables|/Script/Engine.StaticMeshActor|GetStaticMeshComponent _output_get) false)
  (Transformation|AttachActorToActor 0 "None" "SnapToTarget" "SnapToTarget" "KeepWorld" true)
  (Default|CallHammerin))

(event OnComponentEndOverlap(Box)
  (params (OverlappedComponent :type Primitive%20Component%20Object%20Reference) (OtherActor :type Actor%20Object%20Reference) (OtherComp :type Primitive%20Component%20Object%20Reference) (OtherBodyIndex :type Integer))
  ;[1 1 1] Hammer Is removed
  (if (== OtherActor (Variables|Default|GetHammer))
    (Default|CallHammerNotin)
    (Variables|Default|SetDefaultSceneRoot 0)))

(fn ConstructionScript)