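; BP_qkuslic1_calipers is a pair of calipers that a VR motion controller can pick up and drop.
; Pickup swaps to the open mesh, disables physics and snaps it to the attach component at a tuned offset; Drop closes, detaches and restores physics.
; Controller overlap starts a Delay-based poll of grip state that also sets the picked-up flag.
; The hover, drag, use and other interaction functions are stubs returning false.
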(event EventBeginPlay
  (|CallParentFunction) ; This node is disabled and will not be called.\nDrag off pins to build functionality.
)

(event EventPickup
  (params (AttachTo :type Scene%20Component%20Object%20Reference))
  (Components|StaticMesh|SetStaticMesh (Variables|Default|GetStaticMeshComponent) "/Game/Geometry/Meshes/Tools/Calipers_Open.Calipers_Open")
  (Variables|Default|SetARECalipersPickedUp true)
  (Physics|SetSimulatePhysics (Variables|Default|GetStaticMeshComponent) false)
  (Transformation|AttachComponentToComponent (VehicleSound|GetRootComponent) AttachTo "None" "SnapToTarget" "SnapToTarget" "KeepWorld" false)
  (Transformation|SetRelativeLocationAndRotation (Variables|Default|GetStaticMeshComponent) "-2.449041,-0.102751,28.661854" "1.729421,90.491318,9.851128" false false))

(event EventTick
  (params (DeltaSeconds :type Float%20%28single-precision%29))
  (|CallParentFunction DeltaSeconds) ; This node is disabled and will not be called.\nDrag off pins to build functionality.
)

(event Collision|EventActorBeginOverlap
  (params (OtherActor :type Actor%20Object%20Reference))
  (bind _asbp_motion_controller (Utilities|Casting|CastToBP_MotionController OtherActor))
  (if (Utilities|Enum|Equal(Enum) (Variables|/Game/VirtualRealityBP/Blueprints/BP_MotionController.BP_MotionController_C|GetGripState _asbp_motion_controller) "NewEnumerator2") :!label _label
    (Variables|Default|SetARECalipersPickedUp true)
    (else
      (Utilities|FlowControl|Delay 0.2)
      (Utilities|IsValid _asbp_motion_controller
        (:Is%20Valid
          (goto _label))))))

(event EventDrop
  (Components|StaticMesh|SetStaticMesh (Variables|Default|GetStaticMeshComponent) "/Game/Geometry/Meshes/Tools/Calipers_Closed.Calipers_Closed")
  (Variables|Default|SetARECalipersPickedUp false)
  (Physics|SetSimulatePhysics (Variables|Default|GetStaticMeshComponent) true)
  (Transformation|DetachFromActor "KeepWorld" "KeepWorld" "KeepWorld"))

(fn ConstructionScript
  (|CallParentFunction))

(fn CanPickup
  (return false))

(fn OnDragEnd
  (params (Interactor :type World%20Interactor%20Object%20Reference))
  (return false))

(fn OnDragStart
  (params (Interactor :type World%20Interactor%20Object%20Reference))
  (return false))

(fn OnDrag
  (params (Interactor :type World%20Interactor%20Object%20Reference))
  (return false))

(fn OnDrop
  (params (Interactor :type World%20Interactor%20Object%20Reference))
  (return false))

(fn OnPickup
  (params (Interactor :type World%20Interactor%20Object%20Reference))
  (return false))

(fn OnUse
  (params (Interactor :type World%20Interactor%20Object%20Reference))
  (return false))

(fn OnUnHover
  (params (Interactor :type World%20Interactor%20Object%20Reference))
  (return false))

(fn OnHover
  (params (Interactor :type World%20Interactor%20Object%20Reference))
  (return false))